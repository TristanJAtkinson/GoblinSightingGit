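; BP_Mauler is a melee enemy with rat sounds that bites via a sphere trace on a one-second cooldown and awards HUD scrap on death.
; Sighting a TurretTarget-tagged pawn or taking non-lethal damage drives a Behavior Tree blackboard flag, with a Tick-based timer for losing interest.
; LevelConfig compounds health and damage by enemy level through nested checks, while LevelUp raises only damage.
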(event OnSeePawn(PawnSensing)
  (params (Pawn :type Pawn%20Object%20Reference))
  ;[0.2402 1 0.6369] When Player is spotted, change bool value that affects enemy state on BT, and set 'chasetime' to 0
  (if (Actor|ActorHasTag Pawn "TurretTarget")
    (Utilities|FlowControl|DoOnce false
      (:Completed
        (Default|PlayerSeen (Variables|Default|GetWdget%20REF))
        (AI|Components|Blackboard|SetValueasBool (AI|GetBlackboard (AI|GetAIController self)) (Utilities|Name|MakeLiteralName "b_hasseenplayer") true)
        (Variables|PlayerDetection|SetF_chasetime 0.0)
        (CallFunction|ChaseDelay)))))

(event Custom|Chase%20Delay
  ;[0.5948 1 0.2493] If Player has been out of sight for X amount of time, stop chasing
  (if (>= (Variables|PlayerDetection|GetF_chasetime) 1e+01)
    (AI|Components|Blackboard|SetValueasBool (AI|GetBlackboard (AI|GetAIController self)) (Utilities|Name|MakeLiteralName "b_hasseenplayer") false)
    ;[0.2402 1 0.6369] When Player is spotted, change bool value that affects enemy state on BT, and set 'chasetime' to 0
    (Utilities|FlowControl|DoOnce false) ; enters at Reset
  ))

(event Custom|Death
  ;[1 0.655 0.1] Death
  (Utilities|FlowControl|DoOnce false
    (:Completed
      (Audio|PlaySoundatLocation "/Game/Assets/AudioAssets/SFX/Enemies/SC_RatDeath.SC_RatDeath" (Transformation|GetActorLocation) "0, 0, 0" 0.75 1.0 0.0 0 0 0 0)
      (Actor|DestroyActor)
      (bind _foundwidgets (Widget|GetAllWidgetsOfClass "/Game/BluePrints/Widgets/Wb_HUD.Wb_HUD_C" true))
      (Default|IncreaseScrap (Utilities|Array|Get(acopy) _foundwidgets) 650))))

(event Custom|Level%20Up
  ;[0.373 1 0.2038] Level Up
  (Utilities|FlowControl|DoOnce false :!label _label
    (:Completed
      (bind _output_get (Variables|Default|Seti_enemylevel (+ (Variables|Default|Geti_enemylevel) 1)))
      (switch int _output_get
        (:2
          _)
        (:3
          _)
        (:4
          _)
        (:5
          _)
        (:6
          _)
        (:7
          _)
        (:8
          _)
        (:9
          _)
        (:10
          _))
      (Variables|Default|Setf_enemydamage (* (Variables|Default|Getf_enemydamage) 1.1))
      (goto _label Reset))))

(event Custom|Attack
  ;[1 1 1] Melee Attack
  (Utilities|FlowControl|DoOnce false :!label _label
    (:Completed
      (bind _outhit (Collision|SphereTraceByChannel (Transformation|GetWorldLocation (Variables|Default|GetScene1)) (Transformation|GetWorldLocation (Variables|Default|GetScene2)) 1e+02 "TraceTypeQuery2" false 0 "None"))
      (Game|Damage|ApplyDamage (.HitActor (Collision|BreakHitResult _outhit)) (Variables|PawnStats|GetF_EnemyDamage) 0 0)
      (Audio|PlaySoundatLocation "/Game/Assets/AudioAssets/SFX/Enemies/Mauler/SC_RatBite.SC_RatBite" (Transformation|GetActorLocation) "0, 0, 0" 0.75 1.0 0.0 0 0 0 0)
      (Utilities|FlowControl|Delay 1.0)
      (goto _label Reset))))

(event Custom|LevelConfig
  (params (Universal%20Enemy%20Level :type Integer))
  ;[1 0 0] NEED TO LOOK INTO A MORE EFFICIENT WAY OF DOING THIS
  (bind _output_get (Variables|Default|SetI_EnemyLevel Universal%20Enemy%20Level))
  (if (>= _output_get 2)
    (Variables|Default|Setf_enemydamage (* (Variables|Default|Getf_enemydamage) 1.1))
    (Variables|PawnStats|SetF_MaxHP (* (Variables|PawnStats|GetF_MaxHP) 1.1))
    (if (>= _output_get 3)
      (Variables|Default|Setf_enemydamage (* (Variables|Default|Getf_enemydamage) 1.1))
      (Variables|PawnStats|SetF_MaxHP (* (Variables|PawnStats|GetF_MaxHP) 1.1))
      (if (>= _output_get 4)
        (Variables|Default|Setf_enemydamage (* (Variables|Default|Getf_enemydamage) 1.1))
        (Variables|PawnStats|SetF_MaxHP (* (Variables|PawnStats|GetF_MaxHP) 1.1))
        (if (>= _output_get 5)
          (Variables|Default|Setf_enemydamage (* (Variables|Default|Getf_enemydamage) 1.1))
          (Variables|PawnStats|SetF_MaxHP (* (Variables|PawnStats|GetF_MaxHP) 1.1))
          (if (>= _output_get 6)
            (Variables|Default|Setf_enemydamage (* (Variables|Default|Getf_enemydamage) 1.1))
            (Variables|PawnStats|SetF_MaxHP (* (Variables|PawnStats|GetF_MaxHP) 1.1))
            (if (>= _output_get 7)
              (Variables|Default|Setf_enemydamage (* (Variables|Default|Getf_enemydamage) 1.1))
              (Variables|PawnStats|SetF_MaxHP (* (Variables|PawnStats|GetF_MaxHP) 1.1))
              (if (>= _output_get 8)
                (Variables|Default|Setf_enemydamage (* (Variables|Default|Getf_enemydamage) 1.1))
                (Variables|PawnStats|SetF_MaxHP (* (Variables|PawnStats|GetF_MaxHP) 1.1))
                (if (>= _output_get 9)
                  (Variables|Default|Setf_enemydamage (* (Variables|Default|Getf_enemydamage) 1.1))
                  (Variables|PawnStats|SetF_MaxHP (* (Variables|PawnStats|GetF_MaxHP) 1.1))
                  (if (>= _output_get 10)
                    (Variables|Default|Setf_enemydamage (* (Variables|Default|Getf_enemydamage) 1.1))
                    (Variables|PawnStats|SetF_MaxHP (* (Variables|PawnStats|GetF_MaxHP) 1.1)))))))))))
  (Variables|PawnStats|SetF_CurrentHP (Variables|PawnStats|GetF_MaxHP)))

(event Game|Damage|EventAnyDamage
  (params (Damage :type Float%20%28single-precision%29) (DamageType :type Damage%20Type%20Object%20Reference) (InstigatedBy :type Controller%20Object%20Reference) (DamageCauser :type Actor%20Object%20Reference))
  ;[1 0.7569 0.2249] Take Damage
  (bind _output_get (Variables|PawnStats|SetF_CurrentHP (Math|Float|Clamp(Float) (- (Variables|PawnStats|GetF_CurrentHP) Damage) 0.0 (Variables|PawnStats|GetF_MaxHP))))
  (if (<= _output_get 0.0)
    (CallFunction|Death)
    (else
      (if (== (Variables|PlayerDetection|GetF_chasetime) 0.0)
        ;[0.2402 1 0.6369] When Player is spotted, change bool value that affects enemy state on BT, and set 'chasetime' to 0
        (Default|PlayerSeen (Variables|Default|GetWdget%20REF)))
      (AI|Components|Blackboard|SetValueasBool (AI|GetBlackboard (AI|GetAIController self)) (Utilities|Name|MakeLiteralName "b_hasseenplayer") true)
      (Variables|PlayerDetection|SetF_chasetime 0.0)
      (CallFunction|ChaseDelay))))

(event EventTick
  (params (DeltaSeconds :type Float%20%28single-precision%29))
  ;[0.3953 1 0.2782] Amount of time player has been out of sight (resets when spotted)
  (Variables|PlayerDetection|SetF_chasetime (+ (Variables|PlayerDetection|GetF_chasetime) DeltaSeconds)))

(event EventGetWidget
  (params (WdgetREF :type Wb%20HUD%20Object%20Reference))
  (Variables|Default|SetWdget%20REF WdgetREF))

(fn ConstructionScript)