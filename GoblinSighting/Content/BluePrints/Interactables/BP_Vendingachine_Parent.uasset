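; Parent Blueprint for vending machines that sell player upgrades such as health, movement speed, bullet damage and fire rate.
; It binds to the first BP_Power_Switch found, running a timeline that toggles its spotlight and enables interaction once power-up finishes.
; Interface-style functions report power state, prompt text and price.
; Interacting passes the upgrade type to BP_ActionChar and plays a sound, unless the health upgrade limit flag is set.
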(event Custom|Power%20Switch
  (params (On :type Boolean))
  (if On
    (bind (_direction _newtrack_0) (Timeline|Power_TL PlayFromStart)
      (:Update
        (bind _output_get (Variables|Default|SetPower_Alpha _newtrack_0))
        (Rendering|SetVisibility (Variables|Default|GetSpotLight) (select (> _output_get 0.6) true false) false))
      (:Finished
        (switch Utilities|FlowControl|Switch|SwitchonETimelineDirection _direction
          (:Forward
            (Variables|Default|SetCan%20Interact true)
            (Variables|Default|SetPower_On true)))))
    (else
      (Variables|Default|SetCan%20Interact false)
      (Variables|Default|SetPower_On false)
      (Timeline|Power_TL Reverse))))

(event Custom|Power%20On%20Event
  (CallFunction|PowerSwitch true))

(event Custom|Power%20Off%20Event
  (CallFunction|PowerSwitch false))

(event EventOnInteract
  (if (not (Variables|Default|GetUpgrade%20Health%20Limit%20Reached))
    (bind _asbp_action_char (Utilities|Casting|CastToBP_ActionChar (Game|GetPlayerCharacter 0)))
    (Default|AddUpgrade _asbp_action_char self (Variables|Default|GetUpgrade%20Type))
    (Audio|PlaySoundatLocation "/Game/Assets/AudioAssets/SFX/UI/ITEM_UPGRADE.ITEM_UPGRADE" (Transformation|GetActorLocation) "0, 0, 0" 1.0 1.0 0.0 0 0 0 0)))

(event EventBeginPlay
  (bind _outactors (Actor|GetAllActorsOfClass "/Game/BluePrints/Interactables/BP_Power_Switch.BP_Power_Switch_C"))
  (EventDispatchers|BindEventtoTurnonPower (Utilities|Array|Get(acopy) _outactors) (delegate Custom|Power%20On%20Event))
  (EventDispatchers|BindEventtoTurnOffPower (Utilities|Array|Get(acopy) _outactors) (delegate Custom|Power%20Off%20Event)))

(fn ConstructionScript)

(fn CanInteract
  (return (Variables|Default|GetCan%20Interact) true (Variables|Default|GetPower_On)))

(fn IsInteractable/GetDetails
  (return "NewEnumerator3" (Utilities|Text|FormatText "Buy {Upgrade}" (Utilities|Select :Index (Variables|Default|GetUpgrade_Index) :Option%200 "" :Option%201 "Health upgrade" :Option%202 "Movement Speed Upgrade" :Option%203 "Bullet Damage Upgrade" :Option%204 "Fire Rate Upgrade")) (Math|Integer|SelectInt (Variables|Default|GetPrice) 0 (Variables|Default|GetCustom_Price)) (Variables|Default|GetUpgrade_Index)))