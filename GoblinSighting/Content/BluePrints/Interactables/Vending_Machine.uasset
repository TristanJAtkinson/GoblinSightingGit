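; Vending machine interactable that, when its interact event fires, casts the player character to BP_ActionChar and gives it a weapon upgrade.
; It appears unfinished: CanInteract always returns false with no power requirement, and its details report zero price and placeholder "do nothing" text.
; BeginPlay forwards the PowerOn state to PowerSwitch, whose branch has no effect yet, and a second OnInteract event is empty.
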(event Custom|Power%20Switch
  (params (On :type Boolean))
  (if On
    _))

(event EventOnInteract
  (params (Current%20Scrap :type Integer) (Player%20REF :type BP%20Action%20Char%20Object%20Reference))
  (bind _asbp_action_char (Utilities|Casting|CastToBP_ActionChar (Game|GetPlayerCharacter 0)))
  (Default|AddWeaponUpgrade _asbp_action_char 1))

(event EventBeginPlay
  (CallFunction|PowerSwitch (Variables|Default|GetPower_On)))

(event EventOnInteract)

(fn ConstructionScript)

(fn CanInteract
  (return false false))

(fn IsInteractable/GetDetails
  (return "NewEnumerator2" "do nothing" 0 0))