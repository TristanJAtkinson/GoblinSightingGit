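; BP_DoorAli is an interactable door that opens new spawn rooms in GM_GoblinMode.
; On interact, it compares the player's distance to two side markers and flags the far side's room number in SpawnRoomsOpened.
; It then disables interaction, slides the door along Z with a timeline scaled by OpeningTime, and destroys itself.
; Interface functions report its text, price and power requirement, with PowerOn always false.
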(event Custom|Open%20Door
  (bind _door (Variables|Default|GetDoor))
  (bind _relativelocation (Variables|/Script/Engine.SceneComponent|GetRelativeLocation _door))
  (Components|Timeline|SetPlayRate (Variables|Default|GetOpen_DoorTL) (/ 1.0 (Variables|Default|GetOpening_time)))
  (Variables|Default|SetStart%20Location (Variables|/Script/Engine.SceneComponent|GetRelativeLocation (Variables|Default|GetDoor)))
  (Variables|Default|SetEnd_Location (Math|Vector|MakeVector (.x _relativelocation) (.y _relativelocation) (+ (.z _relativelocation) (Variables|Default|GetOpening_Z_Value))))
  (bind _newtrack_0 (Timeline|Open_DoorTL Play)
    (:Update
      (Transformation|SetRelativeLocation (Variables|Default|GetDoor) (Math|Vector|Lerp(Vector) (Variables|Default|GetStart%20Location) (Variables|Default|GetEnd_Location) _newtrack_0) false false))
    (:Finished
      (Actor|DestroyActor))))

(event Custom|On%20Interact_1
  (params (Current%20Scrap :type Integer) (Player%20REF :type BP%20Action%20Char%20Object%20Reference)))

(event EventOnInteract
  (bind _returnvalue (Game|GetPlayerCharacter 0))
  (bind _capsulecomponent (Variables|/Script/Engine.Character|GetCapsuleComponent _returnvalue))
  (bind _returnvalue_2 (Transformation|GetWorldLocation _capsulecomponent))
  (if (< (Math|Vector|Distance(Vector) _returnvalue_2 (Transformation|GetWorldLocation (Variables|Default|Get1))) (Math|Vector|Distance(Vector) _returnvalue_2 (Transformation|GetWorldLocation (Variables|Default|Get2))))
    (bind _asgm_goblin_mode (Utilities|Casting|CastToGM_GoblinMode (Game|GetGameMode)))
    (Utilities|Array|SetArrayElem (Variables|/Game/BluePrints/GM_GoblinMode.GM_GoblinMode_C|GetSpawn_Rooms_Opened _asgm_goblin_mode) (Variables|Default|GetSide2_Room_Number) true true)
    (else
      (bind _asgm_goblin_mode_2 (Utilities|Casting|CastToGM_GoblinMode (Game|GetGameMode)))
      (Utilities|Array|SetArrayElem (Variables|/Game/BluePrints/GM_GoblinMode.GM_GoblinMode_C|GetSpawn_Rooms_Opened _asgm_goblin_mode_2) (Variables|Default|GetSide1_Room_Number) true true)))
  (Variables|Default|SetCan%20Interact false)
  (CallFunction|OpenDoor))

(fn ConstructionScript)

(fn CanInteract
  (return (Variables|Default|GetCan%20Interact) (Variables|Default|GetNeed_Power) false))

(fn IsInteractable/GetDetails
  (return "NewEnumerator2" (Variables|Default|GetText) (Variables|Default|GetPrice) 0))