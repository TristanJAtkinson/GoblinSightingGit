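; Perk vending machine interactable that sells player upgrades, with only the Health Upgrade given a name and default price in its lookups.
; PowerSwitch, turned on at BeginPlay, runs a timeline that toggles the spotlight and enables interaction once power-up finishes.
; Interface functions report power state, prompt text and a price that can be overridden.
; OnInteract passes UpgradeIndex to BP_ActionChar's AddUpgrade without handling payment itself.
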(event Custom|Power%20Switch
  (params (On :type Boolean))
  (if On
    (bind (_direction _newtrack_0) (Timeline|Power_TL PlayFromStart)
      (:Update
        (bind _output_get (Variables|Default|SetPower_Alpha _newtrack_0))
        (Rendering|SetVisibility (Variables|Default|GetSpotLight) (select (> _output_get 0.6) true false) false))
      (:Finished
        (switch Utilities|FlowControl|Switch|SwitchonETimelineDirection _direction
          (:Forward
            (Variables|Default|SetCan%20Interact true)
            (Variables|Default|SetPower_On true)))))
    (else
      (Variables|Default|SetCan%20Interact false)
      (Variables|Default|SetPower_On false)
      (Timeline|Power_TL Reverse))))

(event EventOnInteract
  (bind _asbp_action_char (Utilities|Casting|CastToBP_ActionChar (Game|GetPlayerCharacter 0)))
  (Default|AddUpgrade _asbp_action_char (Variables|Default|GetUpgrade_Index)))

(event EventBeginPlay
  (CallFunction|PowerSwitch true))

(fn ConstructionScript)

(fn CanInteract
  (return (Variables|Default|GetCan%20Interact) true (Variables|Default|GetPower_On)))

(fn IsInteractable/GetDetails
  (return "NewEnumerator3" (Utilities|Text|FormatText "Buy {Perk}" (Utilities|Select :Index (Variables|Default|GetUpgrade_Index) :Option%200 "" :Option%201 "Health Upgrade" :Option%202 "" :Option%203 "")) (Math|Integer|SelectInt (Variables|Default|GetPrice) (Utilities|Select :Index (Variables|Default|GetUpgrade_Index) :Option%200 0 :Option%201 2500 :Option%202 0 :Option%203 0) (Variables|Default|GetCustom_Price)) (Variables|Default|GetUpgrade_Index)))