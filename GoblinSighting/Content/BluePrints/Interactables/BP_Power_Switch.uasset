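; Interactable power switch that offers a "Turn on power" prompt at no cost and requires no existing power.
; Interacting plays a timeline that drives the pivot's rotation to animate the switch.
; When the timeline finishes, it calls the TurnOnPower dispatcher, shows "Power On" on the HUD, then reverses the timeline after a short delay.
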(event Custom|Power%20On
  (bind _newtrack_0 (Timeline|Switch_TL PlayFromStart)
    (:Update
      (Transformation|SetRelativeRotation (Variables|Default|GetPivot) (Math|Rotator|Lerp(Rotator) "0, 0, 0" "0.000000,0.000000,100.000000" _newtrack_0 true) false false)
      (Transformation|SetRelativeRotation (Variables|Default|GetPivot) (Math|Rotator|Lerp(Rotator) "0, 0, 0" "0.000000,0.000000,0.000000" _newtrack_0 true) false false))
    (:Finished
      (Default|CallTurnonPower)
      (bind _foundwidgets (Widget|GetAllWidgetsOfClass "/Game/BluePrints/Widgets/Wb_HUD.Wb_HUD_C" true))
      (Default|AnnouncmentSetText (Utilities|Array|Get(acopy) _foundwidgets) "Power On")
      (Utilities|FlowControl|Delay 0.7)
      (CallFunction|Reverse))))

(event Custom|reverse
  (Development|PrintString "Hello")
  (bind _newtrack_0 (Timeline|Switch_TL ReverseFromEnd)
    (:Update
      (Transformation|SetRelativeRotation (Variables|Default|GetPivot) (Math|Rotator|Lerp(Rotator) "0, 0, 0" "0.000000,0.000000,100.000000" _newtrack_0 true) false false)
      (Transformation|SetRelativeRotation (Variables|Default|GetPivot) (Math|Rotator|Lerp(Rotator) "0, 0, 0" "0.000000,0.000000,0.000000" _newtrack_0 true) false false))
    (:Finished
      (Default|CallTurnonPower)
      (bind _foundwidgets (Widget|GetAllWidgetsOfClass "/Game/BluePrints/Widgets/Wb_HUD.Wb_HUD_C" true))
      (Default|AnnouncmentSetText (Utilities|Array|Get(acopy) _foundwidgets) "Power On")
      (Utilities|FlowControl|Delay 0.7)
      (CallFunction|Reverse))))

(event EventOnInteract
  (Variables|Default|SetType "NewEnumerator0")
  (CallFunction|Poweron))

(fn ConstructionScript)

(fn CanInteract
  (return true false false))

(fn IsInteractable/GetDetails
  (return (Variables|Default|GetType) "Turn on power" 0 0))