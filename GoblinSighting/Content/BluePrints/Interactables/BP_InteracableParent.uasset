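; Base Blueprint for interactable objects that can be gated by player proximity and a scrap cost.
; Actor overlap events with BP_ActionChar set a flag for whether the player is near.
; The interact event stores the player reference only when that flag is set and the supplied scrap meets the requirement.
; The interaction check and detail queries return placeholder defaults, and no scrap is deducted here.
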(event Custom|On%20Interact_1
  (params (Current%20Scrap :type Integer) (Player%20REF :type BP%20Action%20Char%20Object%20Reference))
  (if (and (Variables|Default|GetB_isplayernear) (>= Current%20Scrap (Variables|Default|GetI_requiredscrap)))
    (Variables|Default|SetPlayer%20REF Player%20REF)))

(event Collision|EventActorBeginOverlap
  (params (OtherActor :type Actor%20Object%20Reference))
  (Utilities|Casting|CastToBP_ActionChar OtherActor)
  (Variables|Default|SetB_isplayernear true))

(event Collision|EventActorEndOverlap
  (params (OtherActor :type Actor%20Object%20Reference))
  (Utilities|Casting|CastToBP_ActionChar OtherActor)
  (Variables|Default|SetB_isplayernear false))

(fn ConstructionScript)

(fn CanInteract
  (return false false false))

(fn IsInteractable/GetDetails
  (return "NewEnumerator0" "" 0 0))