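; BP_Door is an interactable door that opens when the player is near and has enough scrap.
; It extends a parent interactable, passing overlap and interact events up, then checks proximity and the scrap requirement on interact.
; A timeline lerps the Cube from the actor location to 300 units above it, with a DoOnce blocking retriggers until it finishes.
; No closing logic or scrap deduction happens in this Blueprint.
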(event EventBeginPlay)

(event Collision|EventActorBeginOverlap
  (params (OtherActor :type Actor%20Object%20Reference))
  (|CallParentFunction OtherActor))

(event Collision|EventActorEndOverlap
  (params (OtherActor :type Actor%20Object%20Reference))
  (|CallParentFunction OtherActor))

(event EventOnInteract
  (params (Current%20Scrap :type Integer))
  (bind _returnvalue (Transformation|GetActorLocation))
  (|CallParentFunction Current%20Scrap)
  (if (and (Variables|Default|GetB_isplayernear) (>= Current%20Scrap (Variables|Default|GetI_requiredscrap)))
    (Utilities|FlowControl|DoOnce false :!label _label
      (:Completed
        (bind _open (Timeline|DoorOpen Play)
          (:Update
            (Transformation|SetWorldLocation (Variables|Default|GetCube) (Math|Vector|Lerp(Vector) _returnvalue (+ _returnvalue "0.000000,0.000000,300.000000") _open) false false))
          (:Finished
            (goto _label Reset)))))))

(fn ConstructionScript
  (|CallParentFunction))