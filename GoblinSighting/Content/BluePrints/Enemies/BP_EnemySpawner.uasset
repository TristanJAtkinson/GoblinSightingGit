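; Enemy spawner that periodically spawns a random BP_Turret or BP_Mauler at a reachable navmesh point around the player.
; Tick accumulates time and compares it to a delay that shortens as the externally set enemy level rises from 1 to 10.
; SpawnEnemies recursively retries when a sampled point is too near the player, but re-samples for the actual spawn location.
; Each new enemy receives the level and widget reference.
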(event Custom|Spawn%20Enemies
  (bind _i_uenemylvl (Variables|Default|GetI_UenemyLvl))
  (bind _wdget_ref (Variables|Default|GetWdget%20REF))
  (if (<= (Math|Vector|Distance(Vector) (.RandomLocation (AI|Navigation|GetRandomReachablePointinRadius (Transformation|GetActorLocation (stale EventBeginPlay _output_get)) 5e+03 0 0)) (Transformation|GetActorLocation (stale EventBeginPlay _output_get))) 5e+02)
    (CallFunction|SpawnEnemies)
    (else
      (switch int (Math|Random|RandomInteger 2)
        (:0
          (bind _returnvalue (Game|SpawnActorfromClass "/Game/BluePrints/Enemies/Turret/BP_Turret.BP_Turret_C" (Math|Conversions|ToTransform(Vector) (.RandomLocation (AI|Navigation|GetRandomReachablePointinRadius (Transformation|GetActorLocation (stale EventBeginPlay _output_get)) 5e+03 0 0))) "Undefined" "MultiplyWithRoot" 0 0))
          (Default|LevelConfig _returnvalue _i_uenemylvl)
          (Default|GetWidget _returnvalue _wdget_ref)
          (Development|PrintString "Turret Spawned"))
        (:1
          (bind _returnvalue_2 (Game|SpawnActorfromClass "/Game/BluePrints/Enemies/Mauler/BP_Mauler.BP_Mauler_C" (Math|Conversions|ToTransform(Vector) (.RandomLocation (AI|Navigation|GetRandomReachablePointinRadius (Transformation|GetActorLocation (stale EventBeginPlay _output_get)) 5e+03 0 0))) "Undefined" "MultiplyWithRoot" 0 0))
          (Default|LevelConfig _returnvalue_2 _i_uenemylvl)
          (Default|GetWidget _returnvalue_2 _wdget_ref)
          (Development|PrintString "Mailer Spawned")))
      (Variables|Default|SetTimeSinceSpawn 0.0))))

(event EventGetUniversalEnemyLevel
  (params (LvL :type Integer))
  (bind _output_get (Variables|Default|SetI_UenemyLvl LvL)))

(event EventGetWidget
  (params (WdgetREF :type Wb%20Crosshair%20Object%20Reference))
  (Variables|Default|SetWdget%20REF WdgetREF))

(event EventGetTimerValue
  (params (Time :type Float%20%28double-precision%29))
  (Variables|Default|SetTime Time))

(event EventTick
  (params (DeltaSeconds :type Float%20%28single-precision%29))
  (bind _output_get (Variables|Default|SetTimeSinceSpawn (+ (Variables|Default|GetTimeSinceSpawn) DeltaSeconds)))
  (switch int (stale EventGetUniversalEnemyLevel _output_get)
    (:1
      (Variables|Default|SetF_SpawnDelay 8.0))
    (:2
      (Variables|Default|SetF_SpawnDelay 7.5))
    (:3
      (Variables|Default|SetF_SpawnDelay 7.0))
    (:4
      (Variables|Default|SetF_SpawnDelay 6.5))
    (:5
      (Variables|Default|SetF_SpawnDelay 6.0))
    (:6
      (Variables|Default|SetF_SpawnDelay 5.5))
    (:7
      (Variables|Default|SetF_SpawnDelay 5.0))
    (:8
      (Variables|Default|SetF_SpawnDelay 4.5))
    (:9
      (Variables|Default|SetF_SpawnDelay 4.0))
    (:10
      (Variables|Default|SetF_SpawnDelay 3.5)))
  (if (> _output_get (Variables|Default|GetF_SpawnDelay))
    (CallFunction|SpawnEnemies)))

(event EventBeginPlay
  (bind _asbp_action_char_base (Utilities|Casting|CastToBP_ActionChar_Base (Game|GetPlayerCharacter 0)))
  (bind _output_get (Variables|Default|SetAs%20BP%20Action%20Char%20Base _asbp_action_char_base)))

(fn ConstructionScript)