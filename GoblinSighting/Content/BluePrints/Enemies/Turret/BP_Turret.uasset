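; Enemy turret that sweeps for pawns tagged TurretTarget and fires BP_Projectile bursts at them.
; Tick runs a Searching/Attacking state machine, rotating a PoseableMesh bone to sweep or, on PawnSensing sightings, face the target.
; A retriggered one-second timer restores searching, while delays pace shots and bursts.
; Damage depletes HP until death plays a random sound and destroys it; enemy level scales a damage variable the projectile spawn never uses.
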(event OnSeePawn(PawnSensing)
  (params (Pawn :type Pawn%20Object%20Reference))
  (bind _poseablemesh (Variables|Default|GetPoseableMesh))
  (if (Actor|ActorHasTag Pawn "TurretTarget")
    (Variables|Targeting|SetTargetLocation (Transformation|GetActorLocation Pawn))
    (Variables|Targeting|SetTurretState "NewEnumerator1")
    (bind _returnvalue (Class|PoseableMeshComponent|GetBoneRotationbyName _poseablemesh "joint2" "WorldSpace"))
    (Components|PoseableMesh|SetBoneRotationbyName _poseablemesh "joint2" (Math|Rotator|MakeRotator (.roll _returnvalue) (.pitch _returnvalue) (- (.yaw (Math|Rotator|FindLookatRotation (Transformation|GetActorLocation) (Variables|Targeting|GetTargetLocation))) -9e+01)) "WorldSpace")
    (Utilities|Time|ClearandInvalidateTimerbyHandle (Variables|Targeting|GetReset%20Turret%20State%20Timer))
    (Utilities|Time|SetTimerbyEvent (delegate Custom|Reset%20Turret%20State) 1.0)))

(event Custom|Death
  (bind _returnvalue (Transformation|GetActorLocation))
  ;[1 0.3642 0.105] Death
  (Utilities|FlowControl|DoOnce false
    (:Completed
      (switch int (Math|Random|RandomInteger 3)
        (:0
          (Audio|PlaySoundatLocation "/Game/AudioAssets/SFX/Enemies/RAT_DEATH_ONE.RAT_DEATH_ONE" _returnvalue "0, 0, 0" 1.0 1.0 0.0 0 0 0 0))
        (:1
          (Audio|PlaySoundatLocation "/Game/AudioAssets/SFX/Enemies/RAT_DEATH_TWO.RAT_DEATH_TWO" _returnvalue "0, 0, 0" 1.0 1.0 0.0 0 0 0 0))
        (:2
          (Audio|PlaySoundatLocation "/Game/AudioAssets/SFX/Enemies/RAT_DEATH_THREE.RAT_DEATH_THREE" _returnvalue "0, 0, 0" 1.0 1.0 0.0 0 0 0 0)))
      (Actor|DestroyActor))))

(event Custom|Rotate%20Turret
  (bind _returnvalue (Utilities|Time|GetWorldDeltaSeconds))
  (bind _returnvalue_2 (* _returnvalue 5e+01))
  (bind _returnvalue_3 (Class|PoseableMeshComponent|GetBoneRotationbyName (Variables|Default|GetPoseableMesh) "joint2" "ComponentSpace"))
  (Variables|Targeting|SetShould%20Turret%20Rotate%20Right (or (and (< (.Yaw (Math|Rotator|BreakRotator _returnvalue_3)) 7e+01) (Variables|Targeting|GetShould%20Turret%20Rotate%20Right)) (and (< (.Yaw (Math|Rotator|BreakRotator _returnvalue_3)) -7e+01) (not (Variables|Targeting|GetShould%20Turret%20Rotate%20Right)))))
  (Components|PoseableMesh|SetBoneRotationbyName (Variables|Default|GetPoseableMesh) "joint2" (Math|Rotator|MakeRotator (.Roll (Math|Rotator|BreakRotator _returnvalue_3)) (.Pitch (Math|Rotator|BreakRotator _returnvalue_3)) (Math|Float|SelectFloat (+ (.Yaw (Math|Rotator|BreakRotator _returnvalue_3)) _returnvalue_2) (- (.Yaw (Math|Rotator|BreakRotator _returnvalue_3)) _returnvalue_2) (Variables|Targeting|GetShould%20Turret%20Rotate%20Right))) "ComponentSpace"))

(event Custom|Level%20Up
  ;[0.373 1 0.2038] Level Up
  (Utilities|FlowControl|DoOnce false :!label _label
    (:Completed
      (bind _output_get (Variables|Default|Seti_enemylevel (+ (Variables|Default|Geti_enemylevel) 1)))
      (switch int _output_get
        (:2
          _)
        (:3
          _)
        (:4
          _)
        (:5
          _)
        (:6
          _)
        (:7
          _)
        (:8
          _)
        (:9
          _)
        (:10
          _))
      (Variables|Default|Setf_enemydamage (* (Variables|Default|Getf_enemydamage) 1.3))
      (goto _label Reset))))

(event Custom|Turret%20Attack
  (bind _arrow (Variables|Default|GetArrow))
  (bind _targetlocation (Variables|Targeting|GetTargetLocation))
  (bind _returnvalue (Transformation|GetWorldLocation _arrow))
  (bind _returnvalue_2 (Math|Vector|GetUnitDirection(Vector) _returnvalue _targetlocation))
  (if (not (Variables|Targeting|GetIsAttacking?))
    (Variables|Targeting|SetIsAttacking? true)
    (bind _returnvalue_3 (Game|SpawnActorfromClass "/Game/BluePrints/Enemies/Turret/BP_Projectile.BP_Projectile_C" (Math|Transform|MakeTransform (+ _returnvalue (* _returnvalue_2 6e+01)) "0, 0, 0" "1.000000,1.000000,1.000000") "Undefined" "MultiplyWithRoot" 0 0))
    (Physics|SetPhysicsLinearVelocity (Variables|/Game/BluePrints/Enemies/Turret/BP_Projectile.BP_Projectile_C|GetSphere _returnvalue_3) (* _returnvalue_2 6e+03) false "None")
    (Utilities|FlowControl|Delay (Variables|Firing|GetDelay%20Between%20individual%20attacks%20in%20second))
    (bind _result (Math|Integer|IncrementInt (Variables|Firing|GetNumber%20of%20Attacks%20Done))
      (:%20%20
        (if (>= _result (Variables|Firing|GetAttack%20Frequency))
          (Variables|Firing|SetNumber%20of%20Attacks%20Done 0)
          (Utilities|FlowControl|Delay (Variables|Firing|GetDelay%20Between%20Multiple%20Attacks%20in%20seconds)))
        (Variables|Targeting|SetIsAttacking? false)))))

(event Custom|Reset%20Turret%20State
  (Variables|Targeting|SetTurretState "NewEnumerator0"))

(event Game|Damage|EventAnyDamage
  (params (Damage :type Float%20%28single-precision%29) (DamageType :type Damage%20Type%20Object%20Reference) (InstigatedBy :type Controller%20Object%20Reference) (DamageCauser :type Actor%20Object%20Reference))
  ;[0.6024 0.5145 0.07535] Recive Damage
  (bind _output_get (Variables|Health|Setf_CurrentHP (- (Variables|Health|Getf_CurrentHP) Damage)))
  (if (<= _output_get 0.0)
    (CallFunction|Death)))

(event EventTick
  (params (DeltaSeconds :type Float%20%28single-precision%29))
  (switch Utilities|FlowControl|Switch|SwitchonTurret_State (Variables|Targeting|GetTurretState)
    (:NewEnumerator0
      (CallFunction|RotateTurret))
    (:NewEnumerator1
      (CallFunction|TurretAttack))))

(event EventBeginPlay
  ;[1 0 0] NEED TO LOOK INTO A MORE EFFICIENT WAY OF DOING THIS
  (if (>= (Variables|Default|Geti_enemylevel) 2)
    (Variables|Default|Setf_enemydamage (* (Variables|Default|Getf_enemydamage) 1.3))
    (if (>= (Variables|Default|Geti_enemylevel) 3)
      (Variables|Default|Setf_enemydamage (* (Variables|Default|Getf_enemydamage) 1.3))
      (if (>= (Variables|Default|Geti_enemylevel) 4)
        (Variables|Default|Setf_enemydamage (* (Variables|Default|Getf_enemydamage) 1.3))
        (if (>= (Variables|Default|Geti_enemylevel) 5)
          (Variables|Default|Setf_enemydamage (* (Variables|Default|Getf_enemydamage) 1.3))
          (if (>= (Variables|Default|Geti_enemylevel) 6)
            (Variables|Default|Setf_enemydamage (* (Variables|Default|Getf_enemydamage) 1.3))
            (if (>= (Variables|Default|Geti_enemylevel) 7)
              (Variables|Default|Setf_enemydamage (* (Variables|Default|Getf_enemydamage) 1.3))
              (if (>= (Variables|Default|Geti_enemylevel) 8)
                (Variables|Default|Setf_enemydamage (* (Variables|Default|Getf_enemydamage) 1.3))
                (if (>= (Variables|Default|Geti_enemylevel) 9)
                  (Variables|Default|Setf_enemydamage (* (Variables|Default|Getf_enemydamage) 1.3))
                  (if (>= (Variables|Default|Geti_enemylevel) 10)
                    _))))))))))

(fn ConstructionScript)