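; BP_TesterT is an enemy turret that sweeps back and forth and fires projectiles at sensed pawns tagged TurretTarget.
; Tick switches between Searching, which oscillates the PoseableMesh Base2 bone's yaw, and Attacking.
; PawnSensing records target location, snaps the base toward it and schedules a one-second return to Searching.
; Attacks launch BP_Projectile from the Arrow via physics velocity, using delays and a counter for burst pacing.
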(event OnSeePawn(PawnSensing)
  (params (Pawn :type Pawn%20Object%20Reference))
  (bind _poseablemesh (Variables|Default|GetPoseableMesh))
  (if (Actor|ActorHasTag Pawn "TurretTarget")
    (Variables|Default|SetTargetLocation (Transformation|GetActorLocation Pawn))
    (Variables|Default|SetTurretState "NewEnumerator1")
    (bind _returnvalue (Class|PoseableMeshComponent|GetBoneRotationbyName _poseablemesh "Base2" "WorldSpace"))
    (Components|PoseableMesh|SetBoneRotationbyName _poseablemesh "Base2" (Math|Rotator|MakeRotator (.roll _returnvalue) (.pitch _returnvalue) (- (.yaw (Math|Rotator|FindLookatRotation (Transformation|GetActorLocation) (Variables|Default|GetTargetLocation))) 9e+01)) "WorldSpace")
    (Utilities|Time|ClearandInvalidateTimerbyHandle (Variables|Default|GetReset%20Turret%20State%20Timer))
    (Utilities|Time|SetTimerbyEvent (delegate Custom|Reset%20Turret%20State) 1.0)))

(event Custom|Rotate%20Turret
  (bind _returnvalue (Utilities|Time|GetWorldDeltaSeconds))
  (bind _returnvalue_2 (* _returnvalue 5e+01))
  (bind _returnvalue_3 (Class|PoseableMeshComponent|GetBoneRotationbyName (Variables|Default|GetPoseableMesh) "Base2" "ComponentSpace"))
  (Variables|Default|SetShould%20Turret%20Rotate%20Right (or (and (< (.Yaw (Math|Rotator|BreakRotator _returnvalue_3)) 7e+01) (Variables|Default|GetShould%20Turret%20Rotate%20Right)) (and (< (.Yaw (Math|Rotator|BreakRotator _returnvalue_3)) -7e+01) (not (Variables|Default|GetShould%20Turret%20Rotate%20Right)))))
  (Components|PoseableMesh|SetBoneRotationbyName (Variables|Default|GetPoseableMesh) "Base2" (Math|Rotator|MakeRotator (.Roll (Math|Rotator|BreakRotator _returnvalue_3)) (.Pitch (Math|Rotator|BreakRotator _returnvalue_3)) (Math|Float|SelectFloat (+ (.Yaw (Math|Rotator|BreakRotator _returnvalue_3)) _returnvalue_2) (- (.Yaw (Math|Rotator|BreakRotator _returnvalue_3)) _returnvalue_2) (Variables|Default|GetShould%20Turret%20Rotate%20Right))) "ComponentSpace"))

(event Custom|Turret%20Attack
  (bind _arrow (Variables|Default|GetArrow))
  (bind _targetlocation (Variables|Default|GetTargetLocation))
  (bind _returnvalue (Transformation|GetWorldLocation _arrow))
  (bind _returnvalue_2 (Math|Vector|GetUnitDirection(Vector) _returnvalue _targetlocation))
  (if (not (Variables|Default|GetIsAttacking?))
    (Variables|Default|SetIsAttacking? true)
    (bind _returnvalue_3 (Game|SpawnActorfromClass "/Game/BluePrints/Enemies/Turret/BP_Projectile.BP_Projectile_C" (Math|Transform|MakeTransform (+ _returnvalue (* _returnvalue_2 6e+01)) "0, 0, 0" "1.000000,1.000000,1.000000") "Undefined" "MultiplyWithRoot" 0 0))
    (Physics|SetPhysicsLinearVelocity (Variables|/Game/BluePrints/Enemies/Turret/BP_Projectile.BP_Projectile_C|GetSphere _returnvalue_3) (* _returnvalue_2 6e+03) false "None")
    (Utilities|FlowControl|Delay (Variables|Default|GetDelay%20Between%20individual%20attacks%20in%20second))
    (bind _result (Math|Integer|IncrementInt (Variables|Default|GetNumber%20of%20Attacks%20Done))
      (:%20%20
        (if (>= _result (Variables|Default|GetAttack%20Frequency))
          (Variables|Default|SetNumber%20of%20Attacks%20Done 0)
          (Utilities|FlowControl|Delay (Variables|Default|GetDelay%20Between%20Multiple%20Attacks%20in%20seconds)))
        (Variables|Default|SetIsAttacking? false)))))

(event Custom|Reset%20Turret%20State
  (Variables|Default|SetTurretState "NewEnumerator0"))

(event EventTick
  (params (DeltaSeconds :type Float%20%28single-precision%29))
  (switch Utilities|FlowControl|Switch|SwitchonTurret_State (Variables|Default|GetTurretState)
    (:NewEnumerator0
      (CallFunction|RotateTurret))
    (:NewEnumerator1
      (CallFunction|TurretAttack))))

(event EventBeginPlay
  (Components|PoseableMesh|SetBoneRotationbyName (Variables|Default|GetPoseableMesh) "Head" "0.000000,-180.000000,0.000000" "ComponentSpace"))

(fn ConstructionScript)